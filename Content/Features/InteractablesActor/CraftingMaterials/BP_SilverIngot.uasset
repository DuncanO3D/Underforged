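; BP_SilverIngot is a silver ingot crafting-material actor that changes its look when heated.
; Its UpdateHeatMesh event swaps the first material slot on MRoot between HeatMaterial_Silver when hot and M_Silver otherwise.
; BeginPlay and the construction script only call the parent, and the overlap and tick events are disabled stubs.
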(event EventBeginPlay
  (|CallParentFunction))

(event Collision|EventActorBeginOverlap
  (params (OtherActor :type Actor%20Object%20Reference))
  (|CallParentFunction OtherActor) ; This node is disabled and will not be called.\nDrag off pins to build functionality.
)

(event EventTick
  (params (DeltaSeconds :type Float%20%28single-precision%29))
  (|CallParentFunction DeltaSeconds) ; This node is disabled and will not be called.\nDrag off pins to build functionality.
)

(event EventUpdateHeatMesh
  (params (_IsHot :type Boolean))
  (if _IsHot
    (Rendering|Material|SetMaterial (Variables|Default|Getm_Root) 0 "/Game/Props/Materials/HeatMaterial_Silver.HeatMaterial_Silver")
    (else
      (Rendering|Material|SetMaterial (Variables|Default|Getm_Root) 0 "/Game/Props/Textures/Metal/M_Silver.M_Silver"))))

(fn ConstructionScript
  (|CallParentFunction))