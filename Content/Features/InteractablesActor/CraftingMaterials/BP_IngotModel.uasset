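; BP_IngotModel is the ingot crafting-material model that gives sound and particle feedback for hammer hit outcomes.
; Cold, no-model and failed hits play only an anvil strike sound at the actor's location.
; Successful and transforming hits set StartHit, play an object strike sound and call SpawnFX, while final hits call only SpawnFX.
; SpawnFX runs the particle system's trails briefly, using a delay to end them.
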(event Custom|Spawn%20FX
  (Effects|Particles|Trails|BeginTrails (Variables|Default|GetParticleSystem) "None" "None" "ETrailWidthMode_FromCentre" 0.0)
  (Utilities|FlowControl|Delay 1.2)
  (Effects|Particles|Trails|EndTrails (Variables|Default|GetParticleSystem)))

(event Custom|OnHitFinalFinal_1
  (CallFunction|SpawnFX))

(event EventOnHitFinal
  (CallFunction|SpawnFX))

(event EventOnHitNoModel
  (Audio|PlaySoundatLocation "/Game/Sound/Forge_sound/HIT_HAMMERONANVIL.HIT_HAMMERONANVIL" (Transformation|GetActorLocation) "0, 0, 0" 1.0 1.0 0.0 0 0 0))

(event EventTick
  (params (DeltaSeconds :type Float%20%28single-precision%29)))

(event EventOnHitSucceeded
  (Variables|Default|SetStartHit true)
  (Audio|PlaySoundatLocation "/Game/Sound/Forge_sound/HIT_HAMMERONOBJECT.HIT_HAMMERONOBJECT" (Transformation|GetActorLocation) "0, 0, 0" 1.0 1.0 0.0 0 0 0)
  (CallFunction|SpawnFX))

(event EventOnHitTransformed
  (Variables|Default|SetStartHit true)
  (Audio|PlaySoundatLocation "/Game/Sound/Forge_sound/HIT_HAMMERONOBJECT.HIT_HAMMERONOBJECT" (Transformation|GetActorLocation) "0, 0, 0" 1.0 1.0 0.0 0 0 0)
  (CallFunction|SpawnFX))

(event EventOnHitWhileCold
  (Audio|PlaySoundatLocation "/Game/Sound/Forge_sound/HIT_HAMMERONANVIL.HIT_HAMMERONANVIL" (Transformation|GetActorLocation) "0, 0, 0" 1.0 1.0 0.0 0 0 0))

(event EventOnHitFailed
  (Audio|PlaySoundatLocation "/Game/Sound/Forge_sound/HIT_HAMMERONANVIL.HIT_HAMMERONANVIL" (Transformation|GetActorLocation) "0, 0, 0" 1.0 1.0 0.0 0 0 0))

(fn ConstructionScript)