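; BP_GoldIngot is a gold ingot crafting-material actor whose look changes with its heat state.
; Its UpdateHeatMesh event takes an IsHot flag and swaps the first material slot of MRoot between a heated gold material and the standard forge gold ingot material.
; The construction script only calls its parent, and the default BeginPlay, overlap and Tick events are disabled.
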(event EventBeginPlay
  (|CallParentFunction) ; This node is disabled and will not be called.\nDrag off pins to build functionality.
)

(event Collision|EventActorBeginOverlap
  (params (OtherActor :type Actor%20Object%20Reference))
  (|CallParentFunction OtherActor) ; This node is disabled and will not be called.\nDrag off pins to build functionality.
)

(event EventTick
  (params (DeltaSeconds :type Float%20%28single-precision%29))
  (|CallParentFunction DeltaSeconds) ; This node is disabled and will not be called.\nDrag off pins to build functionality.
)

(event EventUpdateHeatMesh
  (params (_IsHot :type Boolean))
  (if _IsHot
    (Rendering|Material|SetMaterial (Variables|Default|Getm_Root) 0 "/Game/Props/Materials/HeatMaterial_Gold.HeatMaterial_Gold")
    (else
      (Rendering|Material|SetMaterial (Variables|Default|Getm_Root) 0 "/Game/recup_content_VrSolo/Material/Props/Mt_Instance_Forge_01_Ingot_Gold.Mt_Instance_Forge_01_Ingot_Gold"))))

(fn ConstructionScript
  (|CallParentFunction))