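; BP_FinalProduct_8 is a weapon element final product that plays sound and particle feedback while it is sharpened.
; Each sharpening event plays a sound and refills a short countdown that Tick decrements per frame, showing the sharpening particles until it expires.
; Completion plays an end sound and shows a second particle system, which suppresses the first; a separate event shows that finished effect without sound.
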(event EventTick
  (params (DeltaSeconds :type Float%20%28single-precision%29))
  (if (and (> (Variables|Default|Getsharpening%20value) 0) (not (Variables|/Script/Engine.SceneComponent|GetbVisible (Variables|Default|GetParticleSystem1))))
    (Rendering|SetVisibility (Variables|Default|GetParticleSystem) true false)
    (Math|Integer|DecrementInt (Variables|Default|Getsharpening%20value))
    (else
      (Rendering|SetVisibility (Variables|Default|GetParticleSystem) false false))))

(event EventOnSharpeningDone
  (Audio|PlaySoundatLocation "/Game/Sound/Sharpening/End_sharpening.End_sharpening" (Transformation|GetActorLocation) "0, 0, 0" 1.0 1.0 0.0 0 0 0)
  (Rendering|SetVisibility (Variables|Default|GetParticleSystem1) true false))

(event EventOninSharpening
  (Audio|PlaySoundatLocation "/Game/Sound/Sharpening/On_Sharpening.On_Sharpening" (Transformation|GetActorLocation) "0, 0, 0" 1.0 1.0 0.0 0 0 0)
  (Variables|Default|Setsharpening%20value 3))

(event EventOnFxSharpeningDone
  (Rendering|SetVisibility (Variables|Default|GetParticleSystem1) true false))

(fn ConstructionScript)