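; Interactable hilt mold that reacts visually when water is added.
; OnAddWater shows the Water component, hides it after a short delay, then fires the OnWaterSpread dispatcher.
; Open, close, open/close sound and add-recipe events are empty stubs.
; A similar timed HotLiquid visibility flash is present but disconnected, so it never runs.
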(event Custom|Play%20Sound%20OpenClose)

(event EventBeginPlay)

(event Collision|EventActorBeginOverlap
  (params (OtherActor :type Actor%20Object%20Reference)))

(event EventTick
  (params (DeltaSeconds :type Float%20%28single-precision%29)))

(event EventOnOpen)

(event EventOnClose)

(event EventOnAddRecipe)

(event EventOnAddWater
  (Rendering|SetVisibility (Variables|Default|GetWater) true false)
  (Utilities|FlowControl|Delay 1.5)
  (Rendering|SetVisibility (Variables|Default|GetWater) false false)
  (Default|CallOnWaterSpread))

(fn ConstructionScript)