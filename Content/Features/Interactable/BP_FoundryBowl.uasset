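; BP_FoundryBowl is an interactable foundry bowl that shows molten liquid once heating finishes and plays a pour effect.
; The liquid mesh starts hidden; when heat time ends it appears with the heat material and the bowl is flagged as finished melting.
; Pouring hides the liquid and briefly shows two particle systems for the stream.
; Select, deselect and heat-start events are empty, and the material pickup logic is disconnected.
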(event EventBeginPlay
  (Rendering|SetVisibility (Variables|Default|Getliquid%20mesh) false false))

(event Collision|EventActorBeginOverlap
  (params (OtherActor :type Actor%20Object%20Reference)))

(event EventTick
  (params (DeltaSeconds :type Float%20%28single-precision%29)))

(event EventOnBeginTimeHeat)

(event EventOnEndTimeHeat
  (bind _liquid_mesh (Variables|Default|Getliquid%20mesh))
  (Rendering|SetVisibility _liquid_mesh true false)
  (Rendering|Material|SetMaterial _liquid_mesh 0 "/Game/Props/Materials/HeatMaterial.HeatMaterial")
  (Variables|Default|SetIsFinishMelting true))

(event EventOnDeverseLiquid
  (Rendering|SetVisibility (Variables|Default|Getliquid%20mesh) false false)
  (Rendering|SetVisibility (Variables|Default|GetParticleSystem) true false)
  (Utilities|FlowControl|Delay 2.0)
  (Rendering|SetVisibility (Variables|Default|GetParticleSystem) false false))

(event EventEventSelect)

(event EventEventDeselect)

(fn ConstructionScript)