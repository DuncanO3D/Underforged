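; Draggable bellows actor that animates its skeletal mesh as the player drags it.
; BeginPlay derives a starting height from Angle and the length of Magnitude, and each OnDrag subtracts the vertical drag velocity from it.
; An arcsine converts that height back into an angle, clamped to a small range and written to the AnimBellow anim instance's Rotation on MBone.
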(event EventBeginPlay
  (Variables|Default|Seth (/ (Math|Trig|Sin(Degrees) (Variables|Default|GetAngle)) (Math|Vector|VectorLength (Variables|Default|Getmagnitude)))))

(event Collision|EventActorBeginOverlap
  (params (OtherActor :type Actor%20Object%20Reference)))

(event EventTick
  (params (DeltaSeconds :type Float%20%28single-precision%29)))

(event EventOnDrag
  (params (dragVelocity :type Vector :default "0, 0, 0"))
  (bind _output_get (Variables|Default|Seth (- (Variables|Default|Geth) (.z dragVelocity))))
  (bind _asanim_bellow (Utilities|Casting|CastToAnimBellow (Components|SkeletalMesh|GetAnimInstance (Variables|Default|Getm_bone))))
  (bind _output_get_2 (Variables|Default|SetAngle (Math|Float|Clamp(Float) (Class|KismetMathLibrary|DegAsin (/ _output_get (Math|Vector|VectorLength (Variables|Default|Getmagnitude)))) 0.0 2e+01)))
  (Variables|/Game/Features/Interactable/Dragable/AnimBellow.AnimBellow_C|SetRotation _asanim_bellow (Math|Rotator|MakeRotator 0.0 0.0 _output_get_2)))

(fn ConstructionScript)