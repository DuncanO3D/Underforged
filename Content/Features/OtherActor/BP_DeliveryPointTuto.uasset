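; Tutorial delivery point that displays the current sword order and gives feedback when it succeeds, fails or is not sharpened.
; Shortly after BeginPlay, it writes the sword name, then uses the order's hilt and blade materials to set external instruction texts, colors and GIF visibility.
; Order events trigger particle trails, success also calls OnOrderValidate, and an unsharpened sword shows a timed warning.
; Failure trails stop after a delay, while the success trails' stop logic is unconnected.
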(event Custom|SpawnFXSuccessed
  (Effects|Particles|Trails|BeginTrails (Variables|Default|GetParticleSystem) "None" "None" "ETrailWidthMode_FromCentre" 0.0))

(event Custom|SpawnFXFailed
  (Effects|Particles|Trails|BeginTrails (Variables|Default|GetParticleSystemFailed) "None" "None" "ETrailWidthMode_FromCentre" 0.0)
  (Utilities|FlowControl|Delay 1.2)
  (Effects|Particles|Trails|EndTrails (Variables|Default|GetParticleSystemFailed)))

(event EventOnNotSharpened
  (Rendering|SetVisibility (Variables|Default|GetText%20aiguisage) true false)
  (Utilities|FlowControl|Delay 1e+01)
  (Rendering|SetVisibility (Variables|Default|GetText%20aiguisage) false false))

(event EventOnOrderFailed
  (CallFunction|SpawnFXFailed))

(event EventOnOrderSuccessed
  (CallFunction|SpawnFXSuccessed)
  (Default|CallOnOrderValidate))

(event EventBeginPlay
  (bind _returnvalue (Utilities|Text|MakeLiteralText "Golden horn"))
  (bind _returnvalue_2 (Utilities|Text|MakeLiteralText "Iron crystal"))
  (bind _returnvalue_3 (Utilities|Text|MakeLiteralText "Gold"))
  (bind _returnvalue_4 (Utilities|Text|MakeLiteralText "Iron"))
  (bind _textdoitfairepoignee (Variables|Default|GetTextDoitFairePoignee))
  (bind _textdoitfairelame (Variables|Default|GetTextDoitFaireLame))
  (bind _textrender (Variables|/Script/Engine.TextRenderActor|GetTextRender _textdoitfairepoignee))
  (bind _textrender_2 (Variables|/Script/Engine.TextRenderActor|GetTextRender _textdoitfairelame))
  (Utilities|FlowControl|Delay 0.5)
  (Utilities|FlowControl|Sequence
    (:then_0
      (Rendering|Components|TextRender|SetText (Variables|Default|Getm_orderText) (Utilities|Text|ToText(String) (.m_swordname (Variables|Default|Getm_orderElement)))))
    (:then_1
      (switch string (.m_hiltname (Variables|Default|Getm_orderElement))
        (:Iron
          (Utilities|IsValid _textdoitfairepoignee
            (:Is%20Valid
              (Rendering|Components|TextRender|SetText _textrender _returnvalue_2)
              (Rendering|Components|TextRender|SetTextRenderColor _textrender (Math|Color|MakeColor 0 200 182 255)))
            (:Is%20Not%20Valid
              _))
          (Rendering|Components|TextRender|SetText (Variables|/Script/Engine.TextRenderActor|GetTextRender (Variables|Default|GetIngredient)) _returnvalue_2)
          (Rendering|SetVisibility (Variables|/Script/Engine.Actor|GetRootComponent (Variables|Default|GetMineraiGif)) true false))
        (:Gold
          (Rendering|Components|TextRender|SetText _textrender _returnvalue)
          (Rendering|Components|TextRender|SetTextRenderColor _textrender (Math|Color|MakeColor 0 255 255 255))
          (Rendering|SetVisibility (Variables|/Script/Engine.Actor|GetRootComponent (Variables|Default|GetCorneGif)) true false)
          (Rendering|Components|TextRender|SetText (Variables|/Script/Engine.TextRenderActor|GetTextRender (Variables|Default|GetIngredient)) _returnvalue))))
    (:then_2
      (switch string (.m_bladename (Variables|Default|Getm_orderElement))
        (:Iron
          (Rendering|Components|TextRender|SetText _textrender_2 _returnvalue_4)
          (Rendering|Components|TextRender|SetTextRenderColor _textrender_2 (Math|Color|MakeColor 0 200 182 255))
          (Rendering|SetVisibility (Variables|/Script/Engine.Actor|GetRootComponent (Variables|Default|GetIronIngotGif)) true false)
          (Rendering|Components|TextRender|SetText (Variables|/Script/Engine.TextRenderActor|GetTextRender (Variables|Default|GetLingot)) _returnvalue_4))
        (:Gold
          (Rendering|Components|TextRender|SetText _textrender_2 _returnvalue_3)
          (Rendering|Components|TextRender|SetTextRenderColor _textrender_2 (Math|Color|MakeColor 0 255 255 255))
          (Rendering|SetVisibility (Variables|/Script/Engine.Actor|GetRootComponent (Variables|Default|GetGoldIngotGif)) true false)
          (Rendering|Components|TextRender|SetText (Variables|/Script/Engine.TextRenderActor|GetTextRender (Variables|Default|GetLingot)) _returnvalue_3))))))

(fn ConstructionScript)