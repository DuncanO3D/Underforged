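; BP_ButtonFillWater is a VR push button, named for filling water, that fires when a BP_MotionControllerVR overlaps its StaticMesh.
; The overlap calls PushButton and OnButtonHit, plays an activation sound at world origin, and turns the mesh green.
; After a half-second delay the mesh turns blue and IsPush clears.
; The IsPush-driven lerp that would slide StaticMesh1 in and out is disconnected, so it never runs.
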(event OnComponentBeginOverlap(StaticMesh)
  (params (OverlappedComponent :type Primitive%20Component%20Object%20Reference) (OtherActor :type Actor%20Object%20Reference) (OtherComp :type Primitive%20Component%20Object%20Reference) (OtherBodyIndex :type Integer) (bFromSweep :type Boolean) (SweepResult :type Hit%20Result%20Structure%20%28by%20ref%29))
  (bind _asbp_motion_controller_vr (Utilities|Casting|CastToBP_MotionControllerVR OtherActor))
  (Utilities|IsValid _asbp_motion_controller_vr
    (:Is%20Valid
      (Class|ButtonFillWater|PushButton)
      (Default|CallOnButtonHit)
      (Rendering|Material|SetMaterial (Variables|Default|GetStaticMesh) 0 "/Game/Props/GPE/Magic_portal/Button_green.Button_green")
      (Audio|PlaySoundatLocation "/Game/Sound/Forge_sound/ACTIVATEWATTERBUTTON.ACTIVATEWATTERBUTTON" "0, 0, 0" "0, 0, 0" 1.0 1.0 0.0 0 0 0)
      (Variables|Default|SetIsPush true)
      (Utilities|FlowControl|Delay 0.5)
      (Rendering|Material|SetMaterial (Variables|Default|GetStaticMesh) 0 "/Game/Props/GPE/Magic_portal/Button_blue.Button_blue")
      (Variables|Default|SetIsPush false))))

(event OnComponentBeginOverlap(StaticMesh1)
  (params (OverlappedComponent :type Primitive%20Component%20Object%20Reference) (OtherActor :type Actor%20Object%20Reference) (OtherComp :type Primitive%20Component%20Object%20Reference) (OtherBodyIndex :type Integer) (bFromSweep :type Boolean) (SweepResult :type Hit%20Result%20Structure%20%28by%20ref%29)))

(event EventTick
  (params (DeltaSeconds :type Float%20%28single-precision%29)))

(fn ConstructionScript)