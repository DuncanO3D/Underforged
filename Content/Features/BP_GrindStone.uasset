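; Grindstone actor with a wheel mesh, sound feedback for turning and overlap detection.
; Each Tick calls TryRotate with zero angular speed and, on success, plays the wheel-turning sound at the world origin.
; M_Wheel begin and end overlaps forward the other actor to OnStartActorOverlap and OnEndActorOverlap.
; A countdown for particle visibility is present but disconnected, so it never runs.
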(event OnComponentBeginOverlap(m_Wheel)
  (params (OverlappedComponent :type Primitive%20Component%20Object%20Reference) (OtherActor :type Actor%20Object%20Reference) (OtherComp :type Primitive%20Component%20Object%20Reference) (OtherBodyIndex :type Integer) (bFromSweep :type Boolean) (SweepResult :type Hit%20Result%20Structure%20%28by%20ref%29))
  (Class|GrindStone|OnStartActorOverlap OtherActor))

(event OnComponentEndOverlap(m_Wheel)
  (params (OverlappedComponent :type Primitive%20Component%20Object%20Reference) (OtherActor :type Actor%20Object%20Reference) (OtherComp :type Primitive%20Component%20Object%20Reference) (OtherBodyIndex :type Integer))
  (Class|GrindStone|OnEndActorOverlap OtherActor))

(event EventTick
  (params (DeltaSeconds :type Float%20%28single-precision%29))
  (bind _returnvalue (Class|GrindStone|TryRotate 0.0))
  (if _returnvalue
    (Audio|PlaySoundatLocation "/Game/Sound/Forge_sound/SHARPWHEEL_TURNING_PRELOOPED.SHARPWHEEL_TURNING_PRELOOPED" "0, 0, 0" "0, 0, 0" 1.0 1.0 0.0 0 0 0)))

(fn ConstructionScript)