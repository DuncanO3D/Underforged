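; BP_MicroOnde is a VR microwave prop with a touch button that appears, from its "object sent" sound, to send items placed inside it.
; Box overlaps report InteractableActors through OnTriggerEnter and OnTriggerExit, whose logic lies outside this graph.
; A MotionControllerVR overlapping the button calls OnButtonPressed, then CallOnButtonHit after a short delay.
; The press also runs timed particle trails, plays the sound at world origin and briefly turns the button green.
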(event OnComponentBeginOverlap(Box)
  (params (OverlappedComponent :type Primitive%20Component%20Object%20Reference) (OtherActor :type Actor%20Object%20Reference) (OtherComp :type Primitive%20Component%20Object%20Reference) (OtherBodyIndex :type Integer) (bFromSweep :type Boolean) (SweepResult :type Hit%20Result%20Structure%20%28by%20ref%29))
  (bind _asinteractable_actor (Utilities|Casting|CastToInteractableActor OtherActor))
  (Class|MicroOnde|OnTriggerEnter _asinteractable_actor))

(event OnComponentEndOverlap(Box)
  (params (OverlappedComponent :type Primitive%20Component%20Object%20Reference) (OtherActor :type Actor%20Object%20Reference) (OtherComp :type Primitive%20Component%20Object%20Reference) (OtherBodyIndex :type Integer))
  (bind _asinteractable_actor (Utilities|Casting|CastToInteractableActor OtherActor))
  (Class|MicroOnde|OnTriggerExit _asinteractable_actor))

(event OnComponentBeginOverlap(Button)
  (params (OverlappedComponent :type Primitive%20Component%20Object%20Reference) (OtherActor :type Actor%20Object%20Reference) (OtherComp :type Primitive%20Component%20Object%20Reference) (OtherBodyIndex :type Integer) (bFromSweep :type Boolean) (SweepResult :type Hit%20Result%20Structure%20%28by%20ref%29))
  (bind _asmotion_controller_vr (Utilities|Casting|CastToMotionControllerVR OtherActor))
  (Utilities|FlowControl|Sequence
    (:then_0
      (Class|MicroOnde|OnButtonPressed _asmotion_controller_vr)
      (Utilities|FlowControl|Delay 0.2)
      (Default|CallOnButtonHit))
    (:then_1
      (CallFunction|SpawnFX)
      (Audio|PlaySoundatLocation "/Game/Sound/Forge_sound/OBJECT_SENT.OBJECT_SENT" "0, 0, 0" "0, 0, 0" 1.0 1.0 0.0 0 0 0))
    (:then_2
      (Rendering|Material|SetMaterial (Variables|Default|GetButton) 0 "/Game/Props/GPE/Magic_portal/Button_green.Button_green")
      (Utilities|FlowControl|Delay 0.2)
      (Rendering|Material|SetMaterial (Variables|Default|GetButton) 0 "/Game/Props/GPE/Magic_portal/Button_neutre.Button_neutre"))))

(event Custom|SpawnFX
  (Effects|Particles|Trails|BeginTrails (Variables|Default|GetParticleSystem) "None" "None" "ETrailWidthMode_FromCentre" 0.0)
  (Utilities|FlowControl|Delay 1.2)
  (Effects|Particles|Trails|EndTrails (Variables|Default|GetParticleSystem)))

(fn ConstructionScript)