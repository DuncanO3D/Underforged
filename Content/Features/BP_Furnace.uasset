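; Furnace Blueprint that updates its sound, light, flame particles and text label to match its heating state.
; Each Tick, CanHeat steps the audio volume up or down within 0–1, while MFlameFactor switches the point light and sets a blue "Froid" label when not burning.
; Four particle systems copy the scale of MFlameParticle.
; The red "Chaud" label and sound-playing nodes are disconnected, so nothing here restores the hot label.
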(event EventTick
  (params (DeltaSeconds :type Float%20%28single-precision%29))
  (bind _textrender (Variables|Default|GetTextRender))
  (bind _pointlight (Variables|Default|GetPointLight))
  (bind _audio (Variables|Default|GetAudio))
  (bind _audio_2 (Variables|Default|GetAudio))
  (Utilities|FlowControl|Sequence
    (:then_0
      (if (Class|Furnace|CanHeat)
        (Audio|Components|Audio|SetVolumeMultiplier _audio (Math|Float|Clamp(Float) (+ (Variables|/Script/Engine.AudioComponent|GetVolumeMultiplier _audio) 0.01)) :!class /Script/Engine.AudioComponent)
        (else
          (Audio|Components|Audio|SetVolumeMultiplier _audio_2 (Math|Float|Clamp(Float) (+ (Variables|/Script/Engine.AudioComponent|GetVolumeMultiplier _audio_2) -0.01)) :!class /Script/Engine.AudioComponent))))
    (:then_1
      (if (> (Variables|Default|Getm_flameFactor) 0.0)
        (Rendering|Components|Light|SetIntensity _pointlight 5e+03)
        (else
          (Rendering|Components|TextRender|SetText _textrender (Utilities|Text|ToText(String) "Froid"))
          (Rendering|Components|TextRender|SetTextRenderColor _textrender (Math|Color|MakeColor 255 0 0 255)))))
    (:then_2
      (Transformation|SetRelativeScale3D (Variables|Default|GetParticleSystem1) (Variables|/Script/Engine.SceneComponent|GetRelativeScale3D (Variables|Default|Getm_flameParticle))))
    (:then_3
      (if (== (Variables|Default|Getm_flameFactor) 0.0)
        (Rendering|Components|Light|SetIntensity _pointlight 0.0)))))

(event EventBeginPlay)

(fn ConstructionScript)