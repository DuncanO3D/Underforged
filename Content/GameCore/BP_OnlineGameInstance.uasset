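; Game instance that manages online session hosting, searching, joining and destroying, plus the VR menus leading to them.
; Hosting opens the chosen map as a listen server once the session succeeds, while search results go to the join menu widget.
; Main, host and join widgets are created on first show, given a reference to this instance, cached, then swapped into a registered VR main menu.
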(event Custom|BeginHost
  (params (MapName :type Name) (Target :type Player%20Controller%20Object%20Reference) (PublicConnections :type Integer) (IsLan :type Boolean))
  ;[1 1 1] Network Managment
  ;;[1 1 1] Hosting Session
  (|Session Target PublicConnections IsLan
    (:OnSuccess
      (Game|OpenLevel(byName) MapName true "listen"))))

(event Custom|BeginFindSession
  (params (Target :type Player%20Controller%20Object%20Reference) (MaxResult :type Integer) (IsLan :type Boolean))
  ;[1 1 1] Network Managment
  ;;[1 1 1] Find Session
  (bind _results (|FindSessions Target MaxResult IsLan)
    (:OnSuccess
      (Default|OnSessionSearchCompleated (Variables|Default|GetJoinMenuWidget) _results))))

(event Custom|BeginJoinSession
  (params (Session :type Blueprint%20Session%20Result%20Structure) (Target :type Player%20Controller%20Object%20Reference))
  ;[1 1 1] Network Managment
  ;;[1 1 1] Join Session
  (|JoinSession Target Session))

(event Custom|BeginDestroySession
  (params (Target :type Player%20Controller%20Object%20Reference))
  ;[1 1 1] Network Managment
  ;;[1 1 1] Destroy Session
  (|DestroySession Target))

(event Custom|ShowJoinMenu
  (bind _returnvalue (Game|GetPlayerController 0))
  ;[1 1 1] Menu Managment
  ;;[1 1 1] JoinMenu
  (Utilities|IsValid (Variables|Default|GetJoinMenuWidget)
    (:Is%20Valid
      (CallFunction|AddtoVRMainMenu (Variables|Default|GetJoinMenuWidget)))
    (:Is%20Not%20Valid
      (Utilities|IsValid _returnvalue
        (:Is%20Valid
          (bind _returnvalue_2 (UserInterface|CreateWidget "/Game/HUD/Blueprints/JoinMenuWidget.JoinMenuWidget_C" _returnvalue self))
          (bind _output_get (Variables|Default|SetJoinMenuWidget _returnvalue_2))
          (CallFunction|AddtoVRMainMenu _output_get))))))

(event Custom|ShowHostMenu
  (bind _returnvalue (Game|GetPlayerController 0))
  ;[1 1 1] Menu Managment
  ;;[1 1 1] HostMenu
  (Utilities|IsValid (Variables|Default|GetHostMenuWidget)
    (:Is%20Valid
      (CallFunction|AddtoVRMainMenu (Variables|Default|GetHostMenuWidget)))
    (:Is%20Not%20Valid
      (Utilities|IsValid _returnvalue
        (:Is%20Valid
          (bind _returnvalue_2 (UserInterface|CreateWidget "/Game/HUD/Blueprints/HostMenuWidget.HostMenuWidget_C" _returnvalue self))
          (bind _output_get (Variables|Default|SetHostMenuWidget _returnvalue_2))
          (CallFunction|AddtoVRMainMenu _output_get))))))

(event Custom|ShowMainMenu
  (bind _returnvalue (Game|GetPlayerController 0))
  ;[1 1 1] Menu Managment
  ;;[1 1 1] MainMenu
  (Utilities|IsValid (Variables|Default|GetMainMenuWidget)
    (:Is%20Valid
      (CallFunction|AddtoVRMainMenu (Variables|Default|GetMainMenuWidget)))
    (:Is%20Not%20Valid
      (Utilities|IsValid _returnvalue
        (:Is%20Valid
          (bind _returnvalue_2 (UserInterface|CreateWidget "/Game/HUD/Blueprints/MainMenuWidget.MainMenuWidget_C" _returnvalue self))
          (bind _output_get (Variables|Default|SetMainMenuWidget _returnvalue_2))
          (CallFunction|AddtoVRMainMenu _output_get))))))

(event Custom|RegisterVRMainMenu
  (params (VR_Main_Menu :type VR%20HUD%20Main%20Menu%20Object%20Reference))
  ;[1 1 1] Menu Managment
  (Variables|Default|SetVR_MainMenu VR_Main_Menu))

(fn AddtoVRMainMenu
  (params (Widget :type User%20Widget%20Object%20Reference))
  (Default|ChangeWidget (Variables|Default|GetVR_MainMenu) Widget))