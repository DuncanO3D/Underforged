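; VR game mode that handles player join and leave and the game start and end events.
; After a short post-login delay, it asks every TutoManager to get the right pawn.
; On logout with more than one player in the player array, it destroys the session through BP_OnlineGameInstance and opens the main menu map.
; A successful StartGame sets GameIsRunning, while EndGame has no follow-up logic.
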(event Custom|Start%20Game
  (bind _returnvalue (Class|VRGameMode|StartGame))
  (if _returnvalue
    (Variables|Default|SetGameIsRunning true)))

(event Custom|End%20Game
  (bind _returnvalue (Class|VRGameMode|EndGame))
  (if _returnvalue
    _))

(event EventOnLogout
  (params (ExitingController :type Controller%20Object%20Reference))
  (if (> (Utilities|Array|Length (Variables|/Script/Engine.GameStateBase|GetPlayerArray (Game|GetGameState))) 1)
    (bind _asbp_online_game_instance (Utilities|Casting|CastToBP_OnlineGameInstance (Game|GetGameInstance)))
    (Default|BeginDestroySession _asbp_online_game_instance (Game|GetPlayerController 0))
    (Game|OpenLevel(byName) (Variables|Default|GetMainMenuMapName))))

(event EventPostLogin
  (params (NewPlayer :type Player%20Controller%20Object%20Reference))
  (|CallParentFunction NewPlayer)
  (Utilities|FlowControl|Delay 0.2)
  (bind _outactors (Actor|GetAllActorsOfClass "/Game/GameCore/TutoManager.TutoManager_C"))
  (for _array_element _outactors
    (Default|GetRightPawn _array_element)))

(fn ConstructionScript)